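; Sniper rifle pickup that the third-person character equips by pressing E inside its trigger box.
; Box overlap enables input and shows an interact widget; leaving removes the widget but leaves input enabled.
; Pickup reveals the character's own Gun, attaches to SniperSocket, hides the world Sniper and sets WeaponEquiped.
; If a weapon is already equipped, E plays the firing animation on the character mesh instead.
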(event OnComponentBeginOverlap(Box)
  (params (OverlappedComponent :type Primitive%20Component%20Object%20Reference) (OtherActor :type Actor%20Object%20Reference) (OtherComp :type Primitive%20Component%20Object%20Reference) (OtherBodyIndex :type Integer) (bFromSweep :type Boolean) (SweepResult :type Hit%20Result%20Structure%20%28by%20ref%29))
  ;[1 1 1] Detect player collision for range
  (Variables|Default|Setoverlapping true)
  (Input|EnableInput (Game|GetPlayerController 0))
  (bind _returnvalue (UserInterface|CreateWidget "/Game/Weapon/WBP_SniperInteract.WBP_SniperInteract_C"))
  (bind _output_get (Variables|Default|SetHUD _returnvalue))
  (UserInterface|Viewport|AddtoViewport _output_get 0))

(event OnComponentEndOverlap(Box)
  (params (OverlappedComponent :type Primitive%20Component%20Object%20Reference) (OtherActor :type Actor%20Object%20Reference) (OtherComp :type Primitive%20Component%20Object%20Reference) (OtherBodyIndex :type Integer))
  ;[1 1 1] Detect player collision for range
  (Variables|Default|Setoverlapping false)
  (Input|EnableInput (Game|GetPlayerController 0))
  (Widget|RemovefromParent (Variables|Default|GetHUD)))

(event Input|KeyboardEvents|E
  (params (Key :type Key%20Structure :default "None"))
  ;[1 1 1] Grab sniper
  (:Pressed
    (if (Variables|Default|Getoverlapping)
      (bind _asbp_third_person_character (Utilities|Casting|CastToBP_ThirdPersonCharacter (stale OnComponentBeginOverlap(Box) OtherActor)))
      (bind _output_get (Variables|Default|SetPlayer _asbp_third_person_character))
      (if (Variables|/Game/ThirdPerson/Blueprints/BP_ThirdPersonCharacter.BP_ThirdPersonCharacter_C|GetweaponEquiped _output_get)
        (Components|Animation|PlayAnimation (Variables|/Script/Engine.Character|GetMesh _output_get) "/Game/Animations/GunFiringAnimation.GunFiringAnimation" false)
        (else
          (Rendering|SetVisibility (Variables|/Game/ThirdPerson/Blueprints/BP_ThirdPersonCharacter.BP_ThirdPersonCharacter_C|GetGun _output_get) true true)
          (Transformation|AttachComponentToComponent self (Variables|/Script/Engine.Character|GetMesh _output_get) "SniperSocket" "SnapToTarget" "SnapToTarget" "KeepRelative" true)
          (Rendering|SetVisibility (Variables|Default|GetSniper) false true)
          (Widget|RemovefromParent (Variables|Default|GetHUD))
          (Variables|/Game/ThirdPerson/Blueprints/BP_ThirdPersonCharacter.BP_ThirdPersonCharacter_C|SetweaponEquiped _output_get true))))))

(fn ConstructionScript)